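; Hazard laser actor that repeatedly fires a cylinder beam, starting on BeginPlay or, in trigger mode with a valid TriggerBox, waiting for ActivateLaser.
; A timeline stretches the beam's Z scale, then it holds, hides and repeats after delays, with rise and loop sounds.
; Player kill messages fire once per cycle, only from overlap checks during timeline updates.
; The begin-overlap event only prints debug text.
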(event OnComponentBeginOverlap(Cylinder)
  (params (OverlappedComponent :type Primitive%20Component%20Object%20Reference) (OtherActor :type Actor%20Object%20Reference) (OtherComp :type Primitive%20Component%20Object%20Reference) (OtherBodyIndex :type Integer) (bFromSweep :type Boolean) (SweepResult :type Hit%20Result%20Structure%20%28by%20ref%29))
  (Utilities|Casting|CastToCharacter OtherActor)
  (if (not (Variables|Default|GetNewHidden))
    (Development|PrintString "MORT" true false "(R=1.000000,G=0.000000,B=0.020400,A=1.000000)")))

(event Custom|LaserApparition
  (bind _cylinder (Variables|Default|GetCylinder))
  (bind _scale (Variables|A_Parameter|GetScale))
  (bind (_x _y) (Math|Vector|BreakVector _scale))
  (bind _overlappingactors (Collision|GetOverlappingActors _cylinder "/Game/FirstPerson/Blueprints/BP_FirstPersonCharacter.BP_FirstPersonCharacter_C" :!class /Script/Engine.PrimitiveComponent))
  (bind _output (Utilities|Array|Get(acopy) _overlappingactors))
  (bind _sw1ref (Variables|Default|GetSW1ref)
    (:then
      (Audio|Components|Audio|Stop _sw1ref))
    (:else
      _))
  (Development|SetHiddeninGame (Variables|Default|GetCylinder) false false)
  (bind _returnvalue (Audio|SpawnSoundatLocation "/Game/DragonLD_Template/SOUNDS/S3/DragonLaserRise.DragonLaserRise" (Transformation|GetActorLocation) "0, 0, 0" 1.0 1.0 0.0 0 0))
  (bind _output_get (Variables|Default|SetSW1ref _returnvalue))
  (Audio|Components|Audio|Play _output_get 0.0)
  (bind _laser (Timeline|Timeline PlayFromStart)
    (:Update
      (Transformation|SetWorldScale3D (Variables|Default|GetCylinder) (Math|Vector|MakeVector _x _y (Math|Float|Lerp 0.0 (.Z (Math|Vector|BreakVector _scale)) _laser)))
      (Utilities|IsValid _output
        (:Is%20Valid
          (Utilities|FlowControl|DoOnce false :!label _label
            (:Completed
              (Class|BPITriggerPlayer|Onkillbox(Message) _output))))))
    (:Finished
      (Utilities|FlowControl|Sequence
        (:then_0
          (goto _label Reset))
        (:then_1
          (bind _sw1ref_2 (Variables|Default|GetSW1ref)
            (:then
              (Audio|Components|Audio|Stop _sw1ref_2))
            (:else
              _))
          (bind _returnvalue_2 (Audio|SpawnSoundatLocation "/Game/DragonLD_Template/SOUNDS/S3/DragonLaserLoop.DragonLaserLoop" (Transformation|GetActorLocation) "0, 0, 0" 1.0 1.0 0.0 0 0 false))
          (bind _output_get_2 (Variables|Default|SetSW1ref _returnvalue_2))
          (Audio|Components|Audio|Play _output_get_2 0.0))
        (:then_2
          (Utilities|FlowControl|Delay (Variables|AParameter|GetStayShootTime))
          (Audio|Components|Audio|Stop (Variables|Default|GetSW1ref))
          (Transformation|SetWorldScale3D (Variables|Default|GetCylinder) (Math|Vector|MakeVector 0.0 0.0 0.0))
          (Development|SetHiddeninGame (Variables|Default|GetCylinder) true false)
          (Utilities|FlowControl|Delay (Variables|AParameter|GetWaitToShootTime))
          (CallFunction|LaserApparition))))))

(event EventBeginPlay
  (Components|Timeline|SetPlayRate (Variables|Default|GetTimeline) (/ 1.0 (Variables|AParameter|GetLaserSpd)))
  (if (Variables|AParameter|GetbHaveTrigger?)
    (Utilities|IsValid (Variables|AParameter|GetTriggerBox)
      (:Is%20Valid
        (Development|SetHiddeninGame (Variables|Default|GetCylinder) true false)
        (Variables|Default|SetNewHidden true)))
    (else
      (Utilities|FlowControl|Delay (Variables|AParameter|GetFirstWaitToShoot))
      (CallFunction|LaserApparition))))

(event EventClearLaser
  (Utilities|Time|ClearandInvalidateTimerbyHandle (Variables|Default|GetRefLaser))
  (Actor|DestroyActor))

(event EventActivateLaser
  (bind _cylinder (Variables|Default|GetCylinder))
  (bind _returnvalue (Transformation|GetWorldScale _cylinder))
  (bind (_x _y) (Math|Vector|BreakVector _returnvalue))
  (Development|SetHiddeninGame (Variables|Default|GetCylinder) false false)
  (Transformation|SetWorldScale3D (Variables|Default|GetCylinder) (Math|Vector|MakeVector _x _y 0.0))
  (Utilities|FlowControl|Delay (Variables|AParameter|GetFirstWaitToShoot))
  (CallFunction|LaserApparition))

(fn ConstructionScript
  (Transformation|SetWorldScale3D (Variables|Default|GetCylinder) (Variables|A_Parameter|GetScale))
  (Development|SetHiddeninGame (Variables|Default|GetCylinder) true false))