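; Dragon actor with a periodically blinking laser and a bullet-sensitive weak point.
; A looping timer flip-flops the Cylinder laser and a timeline stretches its Z scale; with a valid trigger box, the timer waits for TriggerTimerEvent.
; Characters touching the visible laser only trigger a "MORT" debug print.
; A bullet hitting the Sphere hides the dragon, teleports it below, stops the timer and calls ClearLaserMessage.
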(event OnComponentBeginOverlap(Cylinder)
  (params (OverlappedComponent :type Primitive%20Component%20Object%20Reference) (OtherActor :type Actor%20Object%20Reference) (OtherComp :type Primitive%20Component%20Object%20Reference) (OtherBodyIndex :type Integer) (bFromSweep :type Boolean) (SweepResult :type Hit%20Result%20Structure%20%28by%20ref%29))
  (Utilities|Casting|CastToCharacter OtherActor)
  (if (not (Variables|Default|GetNewHidden))
    (Development|PrintString "MORT" true false "(R=1.000000,G=0.000000,B=0.020400,A=1.000000)")))

(event OnComponentBeginOverlap(Sphere)
  (params (OverlappedComponent :type Primitive%20Component%20Object%20Reference) (OtherActor :type Actor%20Object%20Reference) (OtherComp :type Primitive%20Component%20Object%20Reference) (OtherBodyIndex :type Integer) (bFromSweep :type Boolean) (SweepResult :type Hit%20Result%20Structure%20%28by%20ref%29))
  (if (== (Utilities|GetClass OtherActor) "/Game/Variant_Shooter/Blueprints/Pickups/Projectiles/BP_ShooterProjectile_Bullet.BP_ShooterProjectile_Bullet_C")
    (Development|PrintString "WEAK POINT HIT" true false "(R=0.000000,G=0.660000,B=1.000000,A=1.000000)" 5.0)
    (Rendering|SetActorHiddenInGame true)
    (Transformation|SetActorLocation "0.000000,0.000000,-1800.000000" false false)
    (Utilities|Time|ClearandInvalidateTimerbyHandle (stale Custom|TriggerTimerEvent _returnvalue_2))
    (Class|BPIDragon|ClearLaser(Message) (Variables|AParameters|GetDesactivateLaserOnHit))))

(event Custom|LaserApparition
  (bind _cylinder (Variables|Default|GetCylinder))
  (bind _returnvalue (Transformation|GetWorldScale _cylinder))
  (bind (_x _y) (Math|Vector|BreakVector _returnvalue))
  (bind _isa (Utilities|FlowControl|FlipFlop)
    (:A
      _)
    (:B
      _))
  (Development|SetHiddeninGame (Variables|Default|GetCylinder) (not _isa) false)
  (Utilities|FlowControl|Sequence
    (:then_0
      (bind _laser (Timeline|Timeline PlayFromStart)
        (:Update
          (Transformation|SetWorldScale3D (Variables|Default|GetCylinder) (Math|Vector|MakeVector _x _y (Math|Float|Lerp 0.0 (.Z (Math|Vector|BreakVector (Variables|A_Parameters|GetScale))) _laser))))))
    (:then_1
      (bind _output_get (Variables|Default|SetNewHidden (not _isa)))
      (if (not _output_get)
        (Utilities|IsValid (Utilities|Array|Get(acopy) (Collision|GetOverlappingActors (Variables|Default|GetCylinder) "/Game/FirstPerson/Blueprints/BP_FirstPersonCharacter.BP_FirstPersonCharacter_C" :!class /Script/Engine.PrimitiveComponent))
          (:Is%20Valid
            (Development|PrintString "MORT" true false "(R=1.000000,G=0.000000,B=0.020400,A=1.000000)")))))))

(event Custom|TriggerTimerEvent
  (bind _cylinder (Variables|Default|GetCylinder))
  (bind _returnvalue (Transformation|GetWorldScale _cylinder))
  (bind (_x _y) (Math|Vector|BreakVector _returnvalue))
  (Development|SetHiddeninGame (Variables|Default|GetCylinder) false false)
  (Transformation|SetWorldScale3D (Variables|Default|GetCylinder) (Math|Vector|MakeVector _x _y 0.0))
  (bind _returnvalue_2 (Utilities|Time|SetTimerbyEvent (delegate Custom|LaserApparition) (Variables|AParameters|GetTime) true)))

(event Custom|SetAnimToLoop
  (params (NewAnimToPlay :type Animation%20Asset%20Object%20Reference))
  (bind _skeletalmesh (Variables|Default|GetSkeletalMesh))
  (Components|Animation|SetAnimation _skeletalmesh NewAnimToPlay)
  (Rendering|SetVisibility _skeletalmesh true false)
  (Development|SetHiddeninGame _skeletalmesh false false))

(event EventBeginPlay
  (Components|Timeline|SetPlayRate (Variables|Default|GetTimeline) (/ 1.0 (Variables|AParameters|GetLaserSpd)))
  (if (Variables|A_Parameters|GetbHaveTrigger?)
    (Utilities|IsValid (Variables|A_Parameters|GetTriggerBox)
      (:Is%20Valid
        (Development|SetHiddeninGame (Variables|Default|GetCylinder) true false)
        (Variables|Default|SetNewHidden true))
      (:Is%20Not%20Valid
        (bind _returnvalue (Utilities|Time|SetTimerbyEvent (delegate Custom|LaserApparition) (Variables|AParameters|GetTime) true :!label _label))))
    (else
      (goto _label))))

(event Game|Damage|EventAnyDamage
  (params (Damage :type Float%20%28single-precision%29) (DamageType :type Damage%20Type%20Object%20Reference) (InstigatedBy :type Controller%20Object%20Reference) (DamageCauser :type Actor%20Object%20Reference)))

(fn ConstructionScript
  (Rendering|SetVisibility (Variables|Default|GetCylinder) false false))