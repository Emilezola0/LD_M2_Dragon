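; Dragon boss actor with two eye weak points and a repeating laser attack.
; Bullet hits on the eyes lower HP; at zero it hides both eyes, stops the laser and notifies its spawn trigger.
; The laser is a timeline-scaled cylinder aimed at random targets or forward, cycled by retriggerable delays with shot and loop sounds.
; Player hits only print "MORT"; a separate timer-driven flip-flop laser with Niagara charge effect also exists.
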(event OnComponentBeginOverlap(Cylinder)
  (params (OverlappedComponent :type Primitive%20Component%20Object%20Reference) (OtherActor :type Actor%20Object%20Reference) (OtherComp :type Primitive%20Component%20Object%20Reference) (OtherBodyIndex :type Integer) (bFromSweep :type Boolean) (SweepResult :type Hit%20Result%20Structure%20%28by%20ref%29))
  (Utilities|Casting|CastToCharacter OtherActor)
  (if (not (Variables|Default|GetNewHidden))
    (Development|PrintString "MORT" true false "(R=1.000000,G=0.000000,B=0.020400,A=1.000000)")))

(event OnComponentBeginOverlap(Dragon_Oeil_L)
  (params (OverlappedComponent :type Primitive%20Component%20Object%20Reference) (OtherActor :type Actor%20Object%20Reference) (OtherComp :type Primitive%20Component%20Object%20Reference) (OtherBodyIndex :type Integer) (bFromSweep :type Boolean) (SweepResult :type Hit%20Result%20Structure%20%28by%20ref%29))
  (if (== (Utilities|GetClass OtherActor) "/Game/Variant_Shooter/Blueprints/Pickups/Projectiles/BP_ShooterProjectile_Bullet.BP_ShooterProjectile_Bullet_C")
    (Math|Float|DecrementFloat (Variables|Default|GetHP)
      (:%20%20
        (Development|SetHiddeninGame (Variables|Default|GetDragon_Oeil_L) true false)
        (Variables|/Script/Engine.PrimitiveComponent|SetbGenerateOverlapEvents (Variables|Default|GetDragon_Oeil_L) false)
        (CallFunction|EVENTISDEADCHECK)))))

(event OnComponentBeginOverlap(Dragon_Oeil_R)
  (params (OverlappedComponent :type Primitive%20Component%20Object%20Reference) (OtherActor :type Actor%20Object%20Reference) (OtherComp :type Primitive%20Component%20Object%20Reference) (OtherBodyIndex :type Integer) (bFromSweep :type Boolean) (SweepResult :type Hit%20Result%20Structure%20%28by%20ref%29))
  (if (== (Utilities|GetClass OtherActor) "/Game/Variant_Shooter/Blueprints/Pickups/Projectiles/BP_ShooterProjectile_Bullet.BP_ShooterProjectile_Bullet_C")
    (Math|Float|DecrementFloat (Variables|Default|GetHP)
      (:%20%20
        (Development|SetHiddeninGame (Variables|Default|GetDragon_Oeil_R) true false)
        (Variables|/Script/Engine.PrimitiveComponent|SetbGenerateOverlapEvents (Variables|Default|GetDragon_Oeil_R) false)
        (CallFunction|EVENTISDEADCHECK)))))

(event Custom|EyeClosedTrigger
  (params (Condition :type Boolean))
  (if Condition
    (Development|SetHiddeninGame (Variables|Default|GetDragon_Oeil_L) true false)
    (Development|SetHiddeninGame (Variables|Default|GetDragon_Oeil_R) true false)
    (Variables|/Script/Engine.PrimitiveComponent|SetbGenerateOverlapEvents (Variables|Default|GetDragon_Oeil_R) false)
    (Variables|/Script/Engine.PrimitiveComponent|SetbGenerateOverlapEvents (Variables|Default|GetDragon_Oeil_L) false)
    (else
      (Development|SetHiddeninGame (Variables|Default|GetDragon_Oeil_L) false false)
      (Development|SetHiddeninGame (Variables|Default|GetDragon_Oeil_R) false false)
      (Variables|/Script/Engine.PrimitiveComponent|SetbGenerateOverlapEvents (Variables|Default|GetDragon_Oeil_R) true)
      (Variables|/Script/Engine.PrimitiveComponent|SetbGenerateOverlapEvents (Variables|Default|GetDragon_Oeil_L) true))))

(event Custom|TriggerTimerEvent
  (bind _cylinder (Variables|Default|GetCylinder))
  (bind _returnvalue (Transformation|GetWorldScale _cylinder))
  (bind (_x _y) (Math|Vector|BreakVector _returnvalue))
  (Development|SetHiddeninGame (Variables|Default|GetCylinder) false false)
  (Transformation|SetWorldScale3D (Variables|Default|GetCylinder) (Math|Vector|MakeVector _x _y 0.0))
  (bind _returnvalue_2 (Utilities|Time|SetTimerbyEvent (delegate Custom|LaserApparition) (Variables|AParameters|GetTime) true)))

(event Custom|SetupDragonLaser
  (params (StartToShoot :type Float%20%28double-precision%29) (WaitToShoot :type Float%20%28double-precision%29) (StayShootTime :type Float%20%28double-precision%29) (bCanKill? :type Boolean) (Targets :type Array%20of%20Actor%20Object%20References) (NewAnimToPlay :type Animation%20Asset%20Object%20Reference))
  ;[0.15 0.15 0.15 0.5] DRAGON ATTACK
  (Variables|SETUP|SetStartToShoot StartToShoot)
  (Variables|SETUP|SetWaitToShoot WaitToShoot)
  (Variables|SETUP|SetStayShootTime StayShootTime)
  (Variables|SETUP|SetbCanKill? bCanKill?)
  (if (> (Utilities|Array|Length Targets) 0)
    (Variables|SETUP|SetTargets Targets))
  (Utilities|FlowControl|Sequence
    (:then_0
      (if (> (Variables|SETUP|GetStartToShoot) 0.5)
        (Audio|PlaySoundatLocation "/Game/DragonLD_Template/SOUNDS/SW_GRR_DRAGON.SW_GRR_DRAGON" (Transformation|GetActorLocation) "0, 0, 0" 1.0 1.0 0.0 0 0 0 0)))
    (:then_1
      (Utilities|FlowControl|RetriggerableDelay (Variables|SETUP|GetStartToShoot))
      (Utilities|IsValid NewAnimToPlay
        (:Is%20Valid
          (CallFunction|SetNewAnim NewAnimToPlay))
        (:Is%20Not%20Valid
          _))
      (CallFunction|DragonLaserwithSetup))))

(event Custom|StopDragonLaser
  ;[0.15 0.15 0.15 0.5] DRAGON ATTACK
  (Variables|Default|SetbCanContinue? false)
  (Development|SetHiddeninGame (Variables|Default|GetCylinder) true false)
  (Transformation|SetWorldScale3D (Variables|Default|GetCylinder) (Math|Vector|MakeVector 0.0 0.0 0.0))
  (bind _soundcueref (Variables|Default|GetSoundCueRef)
    (:then
      (Audio|Components|Audio|Stop _soundcueref))
    (:else)))

(event Custom|ReactivateLasers
  ;[0.15 0.15 0.15 0.5] DRAGON ATTACK
  (Variables|Default|SetbCanContinue? true)
  (Development|SetHiddeninGame (Variables|Default|GetCylinder) false false)
  (Variables|A_Parameters|SetScale (Math|Vector|MakeVector 5.0 5.0 (Math|Vector|Distance(Vector) (Transformation|GetActorLocation (Utilities|Array|Get(acopy) (Variables|SETUP|GetTargets))) (Transformation|GetActorLocation))))
  (Transformation|SetWorldScale3D (Variables|Default|GetCylinder) "0, 0, 0"))

(event Custom|SetAnimToLoop
  (params (NewAnimToPlay :type Animation%20Asset%20Object%20Reference))
  (bind _skeletalmesh (Variables|Default|GetSkeletalMesh))
  (Components|Animation|SetAnimation _skeletalmesh NewAnimToPlay)
  (Rendering|SetVisibility _skeletalmesh true false)
  (Development|SetHiddeninGame _skeletalmesh false false))

(event Custom|SetupBossHP
  (params (HP :type Float%20%28double-precision%29) (SpawnTriggerRef :type BP%20Trigger%20Spawn%20Object%20Reference))
  (Variables|Default|SetHP HP)
  (Variables|Default|SetSpawnTriggerRef SpawnTriggerRef))

(event Custom|LaserApparition
  (bind _cylinder (Variables|Default|GetCylinder))
  (bind _cylinder_2 (Variables|Default|GetCylinder))
  (bind _returnvalue (Transformation|GetWorldScale _cylinder))
  (bind (_x _y) (Math|Vector|BreakVector _returnvalue))
  (bind _isa (Utilities|FlowControl|FlipFlop)
    (:A
      _)
    (:B
      _))
  (Development|SetHiddeninGame (Variables|Default|GetCylinder) (not _isa) false)
  (Utilities|FlowControl|Sequence
    (:then_0
      (bind _returnvalue_2 (Niagara|SpawnSystematLocation "/Game/VFX/NS_Charge.NS_Charge" (Transformation|GetWorldLocation _cylinder_2) (Transformation|GetWorldRotation _cylinder_2)))
      (bind _output_get (Variables|Default|SetNS _returnvalue_2))
      (Effects|Components|ParticleSystem|SetFloatParameter _output_get "ChargeDuration" 0.2)
      (bind _laser (Timeline|Timeline PlayFromStart)
        (:Update
          (Transformation|SetWorldScale3D (Variables|Default|GetCylinder) (Math|Vector|MakeVector _x _y (Math|Float|Lerp 0.0 (.Z (Math|Vector|BreakVector (Variables|A_Parameters|GetScale))) _laser))))
        (:Finished
          (Components|DestroyComponent (Variables|Default|GetNS)))))
    (:then_1
      (bind _output_get_2 (Variables|Default|SetNewHidden (not _isa)))
      (if (not _output_get_2)
        (Utilities|IsValid (Utilities|Array|Get(acopy) (Collision|GetOverlappingActors (Variables|Default|GetCylinder) "/Game/FirstPerson/Blueprints/BP_FirstPersonCharacter.BP_FirstPersonCharacter_C" :!class /Script/Engine.PrimitiveComponent))
          (:Is%20Valid
            (Development|PrintString "MORT" true false "(R=1.000000,G=0.000000,B=0.020400,A=1.000000)")))))))

(event Custom|OLD%20STUFFFOR%20EYE%20HIT
  (Development|PrintString "WEAK POINT HIT" true false "(R=0.000000,G=0.660000,B=1.000000,A=1.000000)" 5.0)
  (Rendering|SetActorHiddenInGame true)
  (Transformation|SetActorLocation "0.000000,0.000000,-1800.000000" false false)
  (Utilities|Time|ClearandInvalidateTimerbyHandle (stale Custom|TriggerTimerEvent _returnvalue_2))
  (Class|BPIDragon|ClearLaser(Message) (Variables|AParameters|GetDesactivateLaserOnHit)))

(event Custom|EVENT_IS_DEAD_CHECK
  (if (<= (Variables|Default|GetHP) 0.0)
    (Variables|Default|SetHP 0.0)
    (Development|SetHiddeninGame (Variables|Default|GetDragon_Oeil_L) true false)
    (Variables|/Script/Engine.PrimitiveComponent|SetbGenerateOverlapEvents (Variables|Default|GetDragon_Oeil_L) false)
    (Development|SetHiddeninGame (Variables|Default|GetDragon_Oeil_R) true false)
    (Variables|/Script/Engine.PrimitiveComponent|SetbGenerateOverlapEvents (Variables|Default|GetDragon_Oeil_R) false)
    (CallFunction|StopDragonLaser)
    (Default|TriggerSpecialAnimonDragonDeath (Variables|Default|GetSpawnTriggerRef))
    (else
      (Development|SetHiddeninGame (Variables|Default|GetDragon_Oeil_L) false false)
      (Variables|/Script/Engine.PrimitiveComponent|SetbGenerateOverlapEvents (Variables|Default|GetDragon_Oeil_L) true)
      (Development|SetHiddeninGame (Variables|Default|GetDragon_Oeil_R) false false)
      (Variables|/Script/Engine.PrimitiveComponent|SetbGenerateOverlapEvents (Variables|Default|GetDragon_Oeil_R) true))))

(event Custom|DragonLaserWithSetup
  (bind _scale (Variables|A_Parameters|GetScale))
  (bind (_x _y) (Math|Vector|BreakVector _scale))
  ;[0.15 0.15 0.15 0.5] DRAGON ATTACK
  (CallFunction|ReactivateLasers)
  (if (<= (Utilities|Array|Length (Variables|SETUP|GetTargets)) 0)
    (Transformation|SetWorldRotation (Variables|Default|GetCylinderPivot) (CallFunction|CylinderForward) false false)
    (else
      (Transformation|SetWorldRotation (Variables|Default|GetCylinderPivot) (CallFunction|RandomTarget) false false)))
  (bind _soundcueref (Variables|Default|GetSoundCueRef)
    (:then
      (Development|PrintString "Hello")
      (Audio|Components|Audio|Stop _soundcueref))
    (:else
      _))
  (Development|SetHiddeninGame (Variables|Default|GetCylinder) false false)
  (bind _returnvalue (Audio|SpawnSoundatLocation "/Game/DragonLD_Template/SOUNDS/S3/DragonLaserShot.DragonLaserShot" (Transformation|GetActorLocation) "0, 0, 0" 1.0 1.0 0.0 0 0))
  (bind _output_get (Variables|Default|SetSoundCueRef _returnvalue))
  (Audio|Components|Audio|Play _output_get 0.0)
  (bind _laser (Timeline|Timeline_2 PlayFromStart)
    (:Update
      (Transformation|SetWorldScale3D (Variables|Default|GetCylinder) (Math|Vector|MakeVector _x _y (Math|Float|Lerp 0.0 (.Z (Math|Vector|BreakVector _scale)) _laser)))
      (Utilities|IsValid (Utilities|Array|Get(acopy) (Collision|GetOverlappingActors (Variables|Default|GetCylinder) "/Game/FirstPerson/Blueprints/BP_FirstPersonCharacter.BP_FirstPersonCharacter_C" :!class /Script/Engine.PrimitiveComponent))
        (:Is%20Valid
          (Utilities|FlowControl|DoOnce false :!label _label
            (:Completed
              (if (and (Variables|SETUP|GetbCanKill?) (Variables|Default|GetbCanContinue?))
                (Development|PrintString "MORT" true false "(R=1.000000,G=0.000000,B=0.020400,A=1.000000)")))))))
    (:Finished
      (Utilities|FlowControl|Sequence
        (:then_0
          (goto _label Reset))
        (:then_1
          (bind _soundcueref_2 (Variables|Default|GetSoundCueRef)
            (:then
              (Audio|Components|Audio|Stop _soundcueref_2))
            (:else
              _))
          (bind _returnvalue_2 (Audio|SpawnSoundatLocation "/Game/DragonLD_Template/SOUNDS/S3/DragonLaserLoop.DragonLaserLoop" (Transformation|GetActorLocation) "0, 0, 0" 1.0 1.0 0.0 0 0 false))
          (bind _output_get_2 (Variables|Default|SetSoundCueRef _returnvalue_2))
          (Audio|Components|Audio|Play _output_get_2 0.0))
        (:then_2
          (Utilities|FlowControl|RetriggerableDelay (Variables|SETUP|GetStayShootTime))
          (if (Variables|Default|GetbCanContinue?)
            (Audio|Components|Audio|Stop (Variables|Default|GetSoundCueRef))
            (Transformation|SetWorldScale3D (Variables|Default|GetCylinder) (Math|Vector|MakeVector 0.0 0.0 0.0))
            (Development|SetHiddeninGame (Variables|Default|GetCylinder) true false)
            (Utilities|FlowControl|RetriggerableDelay (Variables|SETUP|GetWaitToShoot))
            (if (Variables|Default|GetbCanContinue?)
              (CallFunction|DragonLaserwithSetup))))))))

(event EventBeginPlay
  (Utilities|FlowControl|Sequence
    (:then_0
      (Components|Timeline|SetPlayRate (Variables|Default|GetTimeline) (/ 1.0 (Variables|AParameters|GetLaserSpd)))
      (if (Variables|Default|GetEyesClosed?)
        (Development|SetHiddeninGame (Variables|Default|GetDragon_Oeil_L) true false)
        (Development|SetHiddeninGame (Variables|Default|GetDragon_Oeil_R) true false)
        (Variables|/Script/Engine.PrimitiveComponent|SetbGenerateOverlapEvents (Variables|Default|GetDragon_Oeil_R) false)
        (Variables|/Script/Engine.PrimitiveComponent|SetbGenerateOverlapEvents (Variables|Default|GetDragon_Oeil_L) false)
        (else
          (Development|SetHiddeninGame (Variables|Default|GetDragon_Oeil_L) false false)
          (Development|SetHiddeninGame (Variables|Default|GetDragon_Oeil_R) false false)
          (Variables|/Script/Engine.PrimitiveComponent|SetbGenerateOverlapEvents (Variables|Default|GetDragon_Oeil_R) true)
          (Variables|/Script/Engine.PrimitiveComponent|SetbGenerateOverlapEvents (Variables|Default|GetDragon_Oeil_L) true))))
    (:then_1
      (if (Variables|A_Parameters|GetbHaveTrigger?)
        (Utilities|IsValid (Variables|A_Parameters|GetTriggerBox)
          (:Is%20Valid
            _)))
      (Development|SetHiddeninGame (Variables|Default|GetCylinder) true false)
      (Variables|Default|SetNewHidden true))
    (:then_2
      (Rendering|SetActorHiddenInGame true))))

(event Game|Damage|EventAnyDamage
  (params (Damage :type Float%20%28single-precision%29) (DamageType :type Damage%20Type%20Object%20Reference) (InstigatedBy :type Controller%20Object%20Reference) (DamageCauser :type Actor%20Object%20Reference)))

(fn ConstructionScript
  (Rendering|SetVisibility (Variables|Default|GetCylinder) (Variables|AParameters|GetCylinderVISIBILITY) false))

(fn SPAWNROAR
  (bind _sd_roar (Variables|Default|GetSD_ROAR)
    (:then
      (Audio|Components|Audio|Stop _sd_roar))
    (:else
      _))
  (bind _returnvalue (Audio|SpawnSoundatLocation "/Game/DragonLD_Template/SOUNDS/SW_Roar_Dragon.SW_Roar_Dragon" (Transformation|GetActorLocation) "0, 0, 0" 1.0 1.0 0.0 0 0))
  (bind _output_get (Variables|Default|SetSD_ROAR _returnvalue))
  (Audio|Components|Audio|Play _output_get 0.0))

(fn GRRDRAGON
  (bind _sd_rr (Variables|Default|GetSD_RR)
    (:then
      (Audio|Components|Audio|Stop _sd_rr))
    (:else
      _))
  (bind _returnvalue (Audio|SpawnSoundAttached "/Game/DragonLD_Template/SOUNDS/SW_GRR_DRAGON.SW_GRR_DRAGON" (Variables|Default|GetSkeletalMesh) "None" "0, 0, 0" "0, 0, 0" "KeepRelativeOffset" false 1.0 1.0 0.0 0 0))
  (bind _output_get (Variables|Default|SetSD_RR _returnvalue))
  (Audio|Components|Audio|Play _output_get 0.0))

(fn CylinderForward
  (bind _cylinder (Variables|Default|GetCylinder))
  (bind _returnvalue (Transformation|GetWorldLocation _cylinder))
  (return (Math|Rotator|FindLookatRotation _returnvalue (+ _returnvalue (* (Math|Vector|GetForwardVector (Variables|Default|GetCylinderPivot)) 1e+04)))))

(fn RandomTarget
  (return (Math|Rotator|FindLookatRotation (Transformation|GetWorldLocation (Variables|Default|GetCylinder)) (Transformation|GetActorLocation (.OutItem (Utilities|Array|Random (Variables|SETUP|GetTargets)))))))

(fn SetNewAnim
  (params (NewAnimToPlay :type Animation%20Asset%20Object%20Reference))
  (Components|Animation|SetAnimation (Variables|Default|GetSkeletalMesh) NewAnimToPlay))