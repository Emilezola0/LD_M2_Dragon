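; Dragon chase hazard that flies a BP_Dragon along a spline with a laser volume ahead of it that kills overlapping characters.
; Once triggered, a self-rearming frame-delta timer moves dragon and laser, toggling Niagara effects by spline distance.
; Speed scales with laser-to-player distance, rubber-banding the chase.
; A kill resets everything hidden to the spline start; reaching the end hides the dragon and disables killing.
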(event OnComponentBeginOverlap(LASER)
  (params (OverlappedComponent :type Primitive%20Component%20Object%20Reference) (OtherActor :type Actor%20Object%20Reference) (OtherComp :type Primitive%20Component%20Object%20Reference) (OtherBodyIndex :type Integer) (bFromSweep :type Boolean) (SweepResult :type Hit%20Result%20Structure%20%28by%20ref%29))
  (bind _spline (Variables|Default|GetSpline))
  (bind _chararef (Variables|Default|GetCharaRef))
  (bind _ascharacter (Utilities|Casting|CastToCharacter OtherActor))
  (if (Variables|Default|GetbCanDie?)
    (Class|BPITriggerPlayer|Onkillbox(Message) _ascharacter)
    (Variables|Default|SetLOOP? false)
    (Rendering|SetActorHiddenInGame true)
    (Rendering|SetActorHiddenInGame (Variables|Default|GetCharaRef) true)
    (Utilities|Time|ClearandInvalidateTimerbyHandle (stale Custom|TriggerFollowSpline _returnvalue))
    (Variables|Default|SetDistance 0.0)
    (Transformation|SetActorLocation _chararef (+ (Spline|GetLocationatDistanceAlongSpline _spline (Variables|Default|GetDistance) "World") "0.000000,0.000000,400.000000") false false)
    (Transformation|SetActorRotation _chararef (Math|Rotator|CombineRotators (Spline|GetRotationatDistanceAlongSpline _spline (Variables|Default|GetDistance) "World") "0.000000,-90.000000,40.000000"))
    (bind _laser (Variables|Default|GetLASER)
      (:then
        (Transformation|SetWorldLocation _laser (Spline|GetLocationatDistanceAlongSpline _spline (Variables|Default|GetDistance) "World") false false))
      (:else))))

(event Custom|TriggerFollowSpline
  (bind _asbp_dragon (Utilities|Casting|CastToBP_Dragon (Variables|Default|GetCharaRef)))
  (Variables|Default|SetLOOP? true)
  (Rendering|SetActorHiddenInGame _asbp_dragon false)
  (Rendering|SetActorHiddenInGame false)
  (Default|SetAnimtoLoop _asbp_dragon "/Game/Fab/Dragon/prowler_dragon_variant_r_extracted/scene/SkeletalMeshes/Dragon_Roar/DragonVolForward2_Anim_Armature_VolForward_.DragonVolForward2_Anim_Armature_VolForward_")
  (bind _returnvalue (Utilities|Time|SetTimerbyEvent (delegate Custom|UpdateFollowSpline) (Utilities|Time|GetWorldDeltaSeconds)))
  (Variables|Default|SetbCanDie? true))

(event Custom|UpdateFollowSpline
  (bind _chararef (Variables|Default|GetCharaRef))
  (bind _spline (Variables|Default|GetSpline))
  (bind _niagara (Variables|Default|GetNiagara))
  (bind _spline_2 (Variables|Default|GetSpline))
  (Variables|Default|SetDistance (+ (* (Utilities|Time|GetWorldDeltaSeconds) (Variables|Default|GetDragonSpeed)) (Variables|Default|GetDistance)))
  (Transformation|SetActorLocation _chararef (+ (Spline|GetLocationatDistanceAlongSpline _spline_2 (Variables|Default|GetDistance) "World") "0.000000,0.000000,200.000000") false false)
  (Transformation|SetActorRotation _chararef (Math|Rotator|CombineRotators (Spline|GetRotationatDistanceAlongSpline _spline_2 (Variables|Default|GetDistance) "World") "0.000000,-90.000000,25.000000"))
  (bind _laser (Variables|Default|GetLASER)
    (:then
      (Transformation|SetWorldLocation _laser (Spline|GetLocationatDistanceAlongSpline _spline_2 (+ (Variables|Default|GetDistance) 675.0) "World") false false))
    (:else
      _))
  (Utilities|FlowControl|Sequence
    (:then_0
      (if (< (Variables|Default|GetDistance) (Spline|GetSplineLength (Variables|Default|GetSpline)))
        (if (Variables|Default|GetLOOP?) :!label _label
          (CallFunction|TIMEREVENT))
        (else
          ;[0.15 0.15 0.15 0.5] END
          (Rendering|SetActorHiddenInGame (Variables|Default|GetCharaRef) true)
          (Development|SetHiddeninGame _niagara true false)
          (Class|NiagaraComponent|SetAsset _niagara 0 true)
          (Variables|Default|SetbCanDie? false)
          (bind _laser_2 (Variables|Default|GetLASER)
            (:then
              (Development|SetHiddeninGame _laser_2 true false))
            (:else)))))
    (:then_1
      (if (> (Variables|Default|GetDistance) (Spline|GetDistanceAlongSplineatSplinePoint _spline (- (Spline|GetNumberOfSplinePoints _spline) 1)))
        (bind _laser_3 (Variables|Default|GetLASER)
          (:then
            (Components|DestroyComponent _laser_3)
            (goto _label))
          (:else
            (goto _label)))
        (else
          (goto _label))))
    (:then_2
      (if (>= (Variables|Default|GetDistance) (- (Spline|GetDistanceAlongSplineatSplinePoint (Variables|Default|GetSpline) 1) 5e+02))
        (Development|SetHiddeninGame (Variables|Default|GetNiagara) false false)
        (else
          (Development|SetHiddeninGame (Variables|Default|GetNiagara) true false))))
    (:then_3
      (Variables|Default|GetLASER
        (:then
          (Variables|Default|SetDragonSpeed (Math|Float|MapRangeClamped (Math|Vector|Distance(Vector) (Transformation|GetWorldLocation (Variables|Default|GetLASER)) (Transformation|GetActorLocation (Game|GetPlayerCharacter 0))) 0.0 2.5e+03 1e+02 9e+02)))
        (:else)))))

(event Custom|TIMER%20EVENT
  (bind _returnvalue (Utilities|Time|SetTimerbyEvent (delegate Custom|UpdateFollowSpline) (Utilities|Time|GetWorldDeltaSeconds)))
  (Variables|Default|SetbCanDie? true))

(event EventBeginPlay)

(event EventOnkillbox
  (bind _spline (Variables|Default|GetSpline))
  (bind _chararef (Variables|Default|GetCharaRef))
  (Variables|Default|SetLOOP? false)
  (Rendering|SetActorHiddenInGame true)
  (Rendering|SetActorHiddenInGame (Variables|Default|GetCharaRef) true)
  (Utilities|Time|ClearandInvalidateTimerbyHandle (stale Custom|TriggerFollowSpline _returnvalue))
  (Variables|Default|SetDistance 0.0)
  (Transformation|SetActorLocation _chararef (+ (Spline|GetLocationatDistanceAlongSpline _spline (Variables|Default|GetDistance) "World") "0.000000,0.000000,400.000000") false false)
  (Transformation|SetActorRotation _chararef (Math|Rotator|CombineRotators (Spline|GetRotationatDistanceAlongSpline _spline (Variables|Default|GetDistance) "World") "0.000000,-90.000000,40.000000"))
  (bind _laser (Variables|Default|GetLASER)
    (:then
      (Transformation|SetWorldLocation _laser (Spline|GetLocationatDistanceAlongSpline _spline (Variables|Default|GetDistance) "World") false false))
    (:else)))

(fn ConstructionScript
  (Transformation|SetWorldScale3D (Variables|Default|GetLASER) (Variables|Default|GetSCALE%20LASER)))