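; BP_DragonSpawnSpline is an actor that flies a referenced BP_Dragon along a spline.
; TriggerFollowSpline reveals the dragon, loops its flight animation and starts a fast repeating timer.
; Each tick of UpdateFollowSpline advances distance by speed and world delta time, then applies the spline's transform with a height and rotation offset.
; The end-of-spline check that would clear the timer and hide the dragon is disconnected, so it never runs.
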(event Custom|TriggerFollowSpline
  (bind _asbp_dragon (Utilities|Casting|CastToBP_Dragon (Variables|Default|GetCharaRef)))
  (Rendering|SetActorHiddenInGame _asbp_dragon false)
  (Default|SetAnimtoLoop _asbp_dragon "/Game/Fab/Dragon/prowler_dragon_variant_r_extracted/scene/SkeletalMeshes/DRAGON_VOL.DRAGON_VOL")
  (bind _returnvalue (Utilities|Time|SetTimerbyEvent (delegate Custom|UpdateFollowSpline) 0.01 true)))

(event Custom|UpdateFollowSpline
  (bind _spline (Variables|Default|GetSpline))
  (bind _chararef (Variables|Default|GetCharaRef))
  (Variables|Default|SetDistance (+ (* (Utilities|Time|GetWorldDeltaSeconds) (Variables|Default|GetDragonSpeed)) (Variables|Default|GetDistance)))
  (Transformation|SetActorLocation _chararef (+ (Spline|GetLocationatDistanceAlongSpline _spline (Variables|Default|GetDistance) "World") "0.000000,0.000000,400.000000") false false)
  (Transformation|SetActorRotation _chararef (Math|Rotator|CombineRotators (Spline|GetRotationatDistanceAlongSpline _spline (Variables|Default|GetDistance) "World") "0.000000,-90.000000,40.000000")))

(event EventBeginPlay)

(fn ConstructionScript)