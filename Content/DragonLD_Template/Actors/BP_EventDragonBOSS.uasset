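; Event actor that moves a referenced character, apparently the dragon boss, along a spline when triggered.
; TriggerFollowSpline hides the character in game and starts a looping timer.
; Each timer tick advances the distance by DragonSpeed times world delta seconds, then sets the character's location and spline-aligned rotation with a fixed offset.
; The timer clears once the distance reaches the spline's end.
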(event Custom|TriggerFollowSpline
  (Rendering|SetActorHiddenInGame (Variables|Default|GetCharaRef) true)
  (bind _returnvalue (Utilities|Time|SetTimerbyEvent (delegate Custom|UpdateFollowSpline) 0.01 true)))

(event Custom|UpdateFollowSpline
  (bind _spline (Variables|Default|GetSpline))
  (bind _chararef (Variables|Default|GetCharaRef))
  (Variables|Default|SetDistance (+ (* (Utilities|Time|GetWorldDeltaSeconds) (Variables|Default|GetDragonSpeed)) (Variables|Default|GetDistance)))
  (Transformation|SetActorLocation _chararef (Spline|GetLocationatDistanceAlongSpline _spline (Variables|Default|GetDistance) "World") false false)
  (Transformation|SetActorRotation _chararef (Math|Rotator|CombineRotators (Spline|GetRotationatDistanceAlongSpline _spline (Variables|Default|GetDistance) "World") "0.000000,-90.000000,90.000000"))
  (if (not (< (Variables|Default|GetDistance) (Spline|GetSplineLength (Variables|Default|GetSpline))))
    (Utilities|Time|ClearandInvalidateTimerbyHandle (stale Custom|TriggerFollowSpline _returnvalue))))

(event EventBeginPlay)

(fn ConstructionScript)