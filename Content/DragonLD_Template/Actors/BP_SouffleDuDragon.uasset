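; BP_SouffleDuDragon is a dragon's breath laser hazard that periodically switches on and off.
; A looping timer toggles the Cylinder's visibility and replays a Timeline, paced by LaserSpd, that grows its Z scale from zero to the configured Scale.
; While visible, it checks for characters both on switch-on and on overlap begin, and only prints a red "MORT" (death) message on contact.
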(event OnComponentBeginOverlap(Cylinder)
  (params (OverlappedComponent :type Primitive%20Component%20Object%20Reference) (OtherActor :type Actor%20Object%20Reference) (OtherComp :type Primitive%20Component%20Object%20Reference) (OtherBodyIndex :type Integer) (bFromSweep :type Boolean) (SweepResult :type Hit%20Result%20Structure%20%28by%20ref%29))
  (Utilities|Casting|CastToCharacter OtherActor)
  (if (not (Variables|Default|GetNewHidden))
    (Development|PrintString "MORT" true false "(R=1.000000,G=0.000000,B=0.020400,A=1.000000)")))

(event Custom|LaserApparition
  (bind _cylinder (Variables|Default|GetCylinder))
  (bind _returnvalue (Transformation|GetWorldScale _cylinder))
  (bind (_x _y) (Math|Vector|BreakVector _returnvalue))
  (bind _isa (Utilities|FlowControl|FlipFlop)
    (:A
      _)
    (:B
      _))
  (Development|SetHiddeninGame (Variables|Default|GetCylinder) _isa false)
  (Utilities|FlowControl|Sequence
    (:then_0
      (bind _laser (Timeline|Timeline PlayFromStart)
        (:Update
          (Transformation|SetWorldScale3D (Variables|Default|GetCylinder) (Math|Vector|MakeVector _x _y (Math|Float|Lerp 0.0 (.Z (Math|Vector|BreakVector (Variables|A_Parameter|GetScale))) _laser))))))
    (:then_1
      (bind _output_get (Variables|Default|SetNewHidden _isa))
      (if (not _output_get)
        (Utilities|IsValid (Utilities|Array|Get(acopy) (Collision|GetOverlappingActors (Variables|Default|GetCylinder) "/Game/FirstPerson/Blueprints/BP_FirstPersonCharacter.BP_FirstPersonCharacter_C" :!class /Script/Engine.PrimitiveComponent))
          (:Is%20Valid
            (Development|PrintString "MORT" true false "(R=1.000000,G=0.000000,B=0.020400,A=1.000000)")))))))

(event EventBeginPlay
  (Components|Timeline|SetPlayRate (Variables|Default|GetTimeline) (/ 1.0 (Variables|AParameter|GetLaserSpd)))
  (Utilities|Time|SetTimerbyEvent (delegate Custom|LaserApparition) (Variables|AParameter|GetTime) true))

(fn ConstructionScript
  (Transformation|SetWorldScale3D (Variables|Default|GetCylinder) (Variables|A_Parameter|GetScale)))