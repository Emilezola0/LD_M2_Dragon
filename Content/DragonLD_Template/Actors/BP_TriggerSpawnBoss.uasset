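; BP_TriggerSpawnBoss is a one-shot box trigger that stages a dragon boss encounter when a Character enters it.
; It sets the LaserActorRef actor's visibility, switches level sequences and can start laser fire with a roar at a hard-coded transform, immediately or when the sequence finishes.
; Options allow repositioning the actor or pausing a sequence after a delay.
; ResetSpawn re-arms the trigger, and a separate event swaps to the dragon death sequence.
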(event OnComponentBeginOverlap(Box)
  (params (OverlappedComponent :type Primitive%20Component%20Object%20Reference) (OtherActor :type Actor%20Object%20Reference) (OtherComp :type Primitive%20Component%20Object%20Reference) (OtherBodyIndex :type Integer) (bFromSweep :type Boolean) (SweepResult :type Hit%20Result%20Structure%20%28by%20ref%29))
  (bind _laseractorref (Variables|Parameter|Actor|GetLaserActorRef))
  (Utilities|Casting|CastToCharacter OtherActor)
  (Utilities|FlowControl|DoOnce false
    (:Completed
      (switch Utilities|FlowControl|Switch|SwitchonE_PartsSpawnDragon (Variables|Parameter|Box|GetEBoxType)
        (:NewEnumerator5
          (Utilities|FlowControl|Sequence :!label _label
            (:then_0
              (bind _laseractorref_2 (Variables|Parameter|Actor|GetLaserActorRef)
                (:then
                  (Rendering|SetActorHiddenInGame _laseractorref_2 (Variables|Parameter|Actor|GetbActorNewHidden?)))
                (:else)))
            (:then_1
              (Variables|Parameter|Actor|GetLaserActorRef
                (:then
                  (bind _levelsequencertostop (Variables|Parameter|Sequencer|GetLevelSequencerToStop)
                    (:then
                      (if (Variables|Parameter|Sequencer|GetbUsePauseInsteadOfStop?)
                        (Sequencer|Player|Pause (Variables|/Script/LevelSequence.LevelSequenceActor|GetSequencePlayer _levelsequencertostop))
                        (else
                          (Sequencer|Player|Stop (Variables|/Script/LevelSequence.LevelSequenceActor|GetSequencePlayer _levelsequencertostop) :!class /Script/MovieScene.MovieSceneSequencePlayer))))
                    (:else
                      _))
                  (bind _levelsequence (Variables|Parameter|Sequencer|GetLevelSequence)
                    (:then
                      (Sequencer|Player|Play (Variables|/Script/LevelSequence.LevelSequenceActor|GetSequencePlayer _levelsequence) :!class /Script/MovieScene.MovieSceneSequencePlayer)
                      (if (Variables|Parameter|Attack|GetOnSequencerEnd?)
                        (EventDispatchers|AssignOnFinished (Variables|/Script/LevelSequence.LevelSequenceActor|GetSequencePlayer _levelsequence) (delegate Custom|SequencerFinish))
                        (else
                          (if (Variables|Parameter|Attack|GetbUseLaser?) :!label _label_2
                            (Default|StartShooting _laseractorref)
                            (Sequencer|Player|Stop (Variables|/Script/LevelSequence.LevelSequenceActor|GetSequencePlayer (Variables|Parameter|Sequencer|GetLevelSequence)) :!class /Script/MovieScene.MovieSceneSequencePlayer)
                            (Transformation|SetActorLocationAndRotation _laseractorref "28120.000000,-7778.000000,4645.000000" "0.000000,130.000000,0.000000")
                            (Components|Animation|SetAnimation (Variables|/Game/DragonLD_Template/Actors/BP_SpinningLaser.BP_SpinningLaser_C|GetSkeletalMesh _laseractorref) "/Game/Fab/Dragon/prowler_dragon_variant_r_extracted/scene/SkeletalMeshes/Dragon_Roar/DragonRoar3_Anim_PoserRoar.DragonRoar3_Anim_PoserRoar")))))
                    (:else
                      (goto _label_2))))
                (:else)))
            (:then_2
              (if (Variables|Parameter|Attack|Placement|GetbPlaceActorAtLoc?)
                (bind _laseractorref_3 (Variables|Parameter|Actor|GetLaserActorRef)
                  (:then
                    (Transformation|SetActorTransform _laseractorref_3 (Variables|Parameter|Attack|Placement|GetActorNewTransform)))
                  (:else))))))
        (:NewEnumerator0
          (Utilities|FlowControl|Sequence
            (:then_0
              (goto _label))
            (:then_1
              (Utilities|FlowControl|Delay (Variables|Parameter|Sequencer|GetStopOrContinueSequencerAtTime))
              (Sequencer|Player|Pause (Variables|/Script/LevelSequence.LevelSequenceActor|GetSequencePlayer (Variables|Parameter|Sequencer|GetStoppedOrContinuedSequencer))))))))))

(event Custom|TriggerSpecialAnimOnDragonDeath
  ;[0.15 0.15 0.15 0.5] TRIGGER DEATH
  (bind _levelsequence (Variables|Parameter|Sequencer|GetLevelSequence)
    (:then
      (Sequencer|Player|Stop (Variables|/Script/LevelSequence.LevelSequenceActor|GetSequencePlayer _levelsequence) :!class /Script/MovieScene.MovieSceneSequencePlayer)
      (Sequencer|Player|Play (Variables|/Script/LevelSequence.LevelSequenceActor|GetSequencePlayer (Variables|Parameter|Sequencer|GetLevelSequenceOnDragonDeath)) :!class /Script/MovieScene.MovieSceneSequencePlayer))
    (:else)))

(event Custom|ResetSpawn
  (bind _laseractorref (Variables|Parameter|Actor|GetLaserActorRef))
  (Utilities|FlowControl|DoOnce false) ; enters at Reset
)

(event Custom|SequencerFinish
  (bind _laseractorref (Variables|Parameter|Actor|GetLaserActorRef))
  (if (Variables|Parameter|Attack|GetbUseLaser?)
    (Default|StartShooting _laseractorref)
    (Sequencer|Player|Stop (Variables|/Script/LevelSequence.LevelSequenceActor|GetSequencePlayer (Variables|Parameter|Sequencer|GetLevelSequence)) :!class /Script/MovieScene.MovieSceneSequencePlayer)
    (Transformation|SetActorLocationAndRotation _laseractorref "28120.000000,-7778.000000,4645.000000" "0.000000,130.000000,0.000000")
    (Components|Animation|SetAnimation (Variables|/Game/DragonLD_Template/Actors/BP_SpinningLaser.BP_SpinningLaser_C|GetSkeletalMesh _laseractorref) "/Game/Fab/Dragon/prowler_dragon_variant_r_extracted/scene/SkeletalMeshes/Dragon_Roar/DragonRoar3_Anim_PoserRoar.DragonRoar3_Anim_PoserRoar")))

(fn ConstructionScript
  (Components|Box|SetBoxExtent (Variables|Default|GetBox) (Variables|Parameter|Box|GetBoxExtent) true))