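; BP_Trigger is a level trigger box, sized in the construction script, that fires scripted events when a Character overlaps it.
; It activates a laser actor after a delay and clears another immediately, setting an optional actor's visibility in both branches.
; It can also play a delayed world camera shake, and it stops or starts assigned level sequences.
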(event OnComponentBeginOverlap(Box)
  (params (OverlappedComponent :type Primitive%20Component%20Object%20Reference) (OtherActor :type Actor%20Object%20Reference) (OtherComp :type Primitive%20Component%20Object%20Reference) (OtherBodyIndex :type Integer) (bFromSweep :type Boolean) (SweepResult :type Hit%20Result%20Structure%20%28by%20ref%29))
  (bind _levelsequence (Variables|AParameter|GetLevelSequence))
  (Utilities|Casting|CastToCharacter OtherActor)
  (Utilities|FlowControl|Sequence
    (:then_0
      (Utilities|FlowControl|Delay (Variables|AParameter|GetTimeToActivate))
      (Class|BPIDragon|ActivateLaser(Message) (Variables|AParameter|GetActiveLaserActor))
      (bind _showorhideactor (Variables|AParameter|GetShowOrHideActor)
        (:then
          (Rendering|SetActorHiddenInGame _showorhideactor (Variables|AParameter|GetbActorNewHIdden?)))
        (:else)))
    (:then_1
      (if (Variables|AParameter|GetbPlayCameraShake?)
        (Utilities|FlowControl|Delay (Variables|AParameter|GetCameraShakeTimeToActivate))
        (Camera|PlayWorldCameraShake "/Game/DragonLD_Template/Actors/BP_CameraShakeBase.BP_CameraShakeBase_C" (Transformation|GetActorLocation) 2e+02 5e+03)))
    (:then_2
      (bind _stopsequence (Variables|AParameter|GetStopSequence)
        (:then
          (Sequencer|Player|Stop (Variables|/Script/LevelSequence.LevelSequenceActor|GetSequencePlayer _stopsequence) :!class /Script/MovieScene.MovieSceneSequencePlayer))
        (:else
          _))
      (Utilities|IsValid _levelsequence
        (:Is%20Valid
          (Sequencer|Player|Play (Variables|/Script/LevelSequence.LevelSequenceActor|GetSequencePlayer _levelsequence) :!class /Script/MovieScene.MovieSceneSequencePlayer))))
    (:then_3
      (Class|BPIDragon|ClearLaser(Message) (Variables|AParameter|GetClearLaserActor))
      (bind _showorhideactor_2 (Variables|AParameter|GetShowOrHideActor)
        (:then
          (Rendering|SetActorHiddenInGame _showorhideactor_2 (Variables|AParameter|GetbActorNewHIdden?)))
        (:else)))))

(fn ConstructionScript
  (Components|Box|SetBoxExtent (Variables|Default|GetBox) (Variables|AParameter|GetBoxExtent) true))