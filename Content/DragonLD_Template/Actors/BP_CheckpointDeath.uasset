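; BP_CheckpointDeath is a trigger volume actor that acts as either a kill zone or a checkpoint, depending on its KillZone flag.
; When a Character overlaps its box, it sends that character either a killbox message or a checkpoint message.
; The checkpoint message carries the actor's location and the arrow component's world rotation.
; The construction script sizes the box from an extent variable.
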(event OnComponentBeginOverlap(Box)
  (params (OverlappedComponent :type Primitive%20Component%20Object%20Reference) (OtherActor :type Actor%20Object%20Reference) (OtherComp :type Primitive%20Component%20Object%20Reference) (OtherBodyIndex :type Integer) (bFromSweep :type Boolean) (SweepResult :type Hit%20Result%20Structure%20%28by%20ref%29))
  (bind _ascharacter (Utilities|Casting|CastToCharacter OtherActor))
  (if (Variables|Default|GetKillZone)
    (Class|BPITriggerPlayer|Onkillbox(Message) _ascharacter)
    (else
      (Class|BPITriggerPlayer|Checkpoint(Message) _ascharacter (Transformation|GetActorLocation) (Transformation|GetWorldRotation (Variables|Default|GetArrow))))))

(event EventBeginPlay)

(event Collision|EventActorBeginOverlap
  (params (OtherActor :type Actor%20Object%20Reference)))

(event EventTick
  (params (DeltaSeconds :type Float%20%28single-precision%29)))

(fn ConstructionScript
  (Components|Box|SetBoxExtent (Variables|Default|GetBox) (Variables|Default|GetIn%20Box%20Extent) true))