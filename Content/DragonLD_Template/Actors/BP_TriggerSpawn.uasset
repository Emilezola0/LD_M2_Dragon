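; BP_TriggerSpawn is a trigger volume actor that starts a scripted dragon moment when a Character enters it.
; Its Box overlap plays the referenced Level Sequence and binds to the player's OnFinished event.
; When the sequence finishes, it calls ShootAtLocation on the DragonActiveRolePlay reference.
; The construction script sizes the Box from a BoxExtent variable; nothing in the logic guards against repeated triggering.
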(event OnComponentBeginOverlap(Box)
  (params (OverlappedComponent :type Primitive%20Component%20Object%20Reference) (OtherActor :type Actor%20Object%20Reference) (OtherComp :type Primitive%20Component%20Object%20Reference) (OtherBodyIndex :type Integer) (bFromSweep :type Boolean) (SweepResult :type Hit%20Result%20Structure%20%28by%20ref%29))
  (bind _levelsequence (Variables|AParameter|GetLevelSequence))
  (bind _sequenceplayer (Variables|/Script/LevelSequence.LevelSequenceActor|GetSequencePlayer _levelsequence))
  (Utilities|Casting|CastToCharacter OtherActor)
  (Sequencer|Player|Play _sequenceplayer :!class /Script/MovieScene.MovieSceneSequencePlayer)
  (EventDispatchers|AssignOnFinished _sequenceplayer (delegate Custom|OnFinished_Event)))

(event Custom|OnFinished_Event
  (Default|ShootatLocation (Variables|AParameter|GetDragonActiveRolePlay)))

(fn ConstructionScript
  (Components|Box|SetBoxExtent (Variables|Default|GetBox) (Variables|AParameter|GetBoxExtent) true))