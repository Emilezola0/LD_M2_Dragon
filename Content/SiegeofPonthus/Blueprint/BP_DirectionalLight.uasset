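; BP_DirectionalLight is a combined environment lighting actor that bundles a directional light, sky light, exponential height fog and post process in one placeable Blueprint.
; Its Construction Script copies exposed variables onto each component, covering shadows, light shafts, light functions, ray tracing and volumetric fog.
; The sky light recaptures after its settings are applied, and a single settings struct drives the post process.
; The event graph holds only disabled stub events, so there is no runtime logic.
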(event EventBeginPlay)

(event Collision|EventActorBeginOverlap
  (params (OtherActor :type Actor%20Object%20Reference)))

(event EventTick
  (params (DeltaSeconds :type Float%20%28single-precision%29)))

(fn ConstructionScript
  (bind _directionallight (Variables|Default|GetDirectionalLight))
  (bind _skylight (Variables|Default|GetSkyLight))
  (bind _exponentialheightfog (Variables|Default|GetExponentialHeightFog))
  (Utilities|FlowControl|Sequence
    (:then_0
      ;[1 1 1] Directional Light
      (Transformation|SetMobility _directionallight (Variables|DIRECTIONALLIGHT|GetDirecitonal%20Mobility))
      (Rendering|Components|Light|SetCastShadows _directionallight (Variables|DIRECTIONALLIGHT|GetDirectional%20Cast%20Shadow))
      (Class|LightComponentBase|SetCastRaytracedShadow _directionallight (Variables|DIRECTIONALLIGHT|GetDirectional%20Cast%20Raytraced%20Shadows))
      (Rendering|Components|Light|SetIntensity _directionallight (Variables|DIRECTIONALLIGHT|GetDirectional%20Intensity))
      (Class|LightComponent|SetVolumetricScatteringIntensity _directionallight (Variables|DIRECTIONALLIGHT|GetDirectional%20Volumetric%20Intensity))
      (Rendering|Components|Light|SetLightColor _directionallight (Variables|DIRECTIONALLIGHT|GetDirectional%20Color) (Variables|DIRECTIONALLIGHT|GetUse%20SRGB%20Color%20For%20Directional))
      (Class|LightComponent|SetIndirectLightingIntensity _directionallight (Variables|DIRECTIONALLIGHT|GetDirectional%20Indirect%20Lighting%20Intensity))
      (Class|LightComponent|SetShadowBias _directionallight (Variables|DIRECTIONALLIGHT|GetDirectional%20Shadow%20Bias))
      (Class|LightComponentBase|SetSamplesPerPixel _directionallight (Variables|DIRECTIONALLIGHT|GetDirectional%20Raytrace%20Samples%20Per%20Pixel))
      (Class|DirectionalLightComponent|SetEnableLightShaftOcclusion _directionallight (Variables|DIRECTIONALLIGHT|GetEnable%20Light%20Shaft%20Occlusion))
      (Class|DirectionalLightComponent|SetOcclusionMaskDarkness _directionallight (Variables|DIRECTIONALLIGHT|GetOcclusion%20Mask%20Darkness))
      (Class|LightComponent|SetEnableLightShaftBloom _directionallight (Variables|DIRECTIONALLIGHT|GetEnable%20Light%20Shaft%20Bloom))
      (Class|LightComponent|SetBloomScale _directionallight (Variables|DIRECTIONALLIGHT|GetLight%20Shaft%20Bloom%20Scale))
      (Class|LightComponent|SetBloomThreshold _directionallight (Variables|DIRECTIONALLIGHT|GetLight%20Shaft%20Bloom%20Threshold))
      (Class|LightComponent|SetBloomTint _directionallight (Variables|DIRECTIONALLIGHT|GetLight%20Shaft%20Bloom%20Tint))
      (Class|DirectionalLightComponent|SetDynamicShadowCascades _directionallight (Variables|DIRECTIONALLIGHT|GetDynamic%20Shadow%20Cascades))
      (Class|LightComponent|SetAffectTranslucentLighting _directionallight (Variables|DIRECTIONALLIGHT|GetAffect%20Translucent%20Lighting))
      (Class|LightComponentBase|SetAffectReflection _directionallight (Variables|DIRECTIONALLIGHT|GetAffect%20Reflections))
      (Rendering|SetVisibility _directionallight (Variables|DIRECTIONALLIGHT|GetSet%20Directional%20Visibilty) false)
      (Development|SetHiddeninGame _directionallight (Variables|DIRECTIONALLIGHT|GetHidden%20In%20Game) false)
      (Class|DirectionalLightComponent|SetDynamicShadowDistanceStationaryLight _directionallight (Variables|DIRECTIONALLIGHT|GetDynamic%20Shadow%20Distance%20For%20Stationary%20Mode))
      (Class|DirectionalLightComponent|SetDynamicShadowDistanceMovableLight _directionallight (Variables|DIRECTIONALLIGHT|GetDynamic%20Shadow%20Distance%20For%20Movable%20Mode))
      (Class|DirectionalLightComponent|SetCascadeDistributionExponent _directionallight (Variables|DIRECTIONALLIGHT|GetDistribution%20Exponent))
      (Class|DirectionalLightComponent|SetCascadeTransitionFraction _directionallight (Variables|DIRECTIONALLIGHT|GetTransition%20Fraction))
      (Class|DirectionalLightComponent|SetShadowDistanceFadeoutFraction _directionallight (Variables|DIRECTIONALLIGHT|GetDistance%20Fadeout%20Fraction))
      (Rendering|Components|Light|SetLightFunctionMaterial _directionallight (Variables|DIRECTIONALLIGHT|GetLight%20Function))
      (Class|LightComponent|SetLightFunctionScale _directionallight (Variables|DIRECTIONALLIGHT|GetLight%20Function%20Scale))
      (Class|LightComponent|SetLightFunctionFadeDistance _directionallight (Variables|DIRECTIONALLIGHT|GetLight%20Function%20Fade%20Distance))
      (Class|LightComponent|SetLightFunctionDisabledBrightness _directionallight (Variables|DIRECTIONALLIGHT|GetLight%20Function%20Disabled%20Brightness)))
    (:then_1
      ;[1 1 1] Skylight
      (Transformation|SetMobility _skylight (Variables|SKYLIGHT|GetSkylight%20Mobility))
      (Rendering|Components|Light|SetCastShadows _skylight (Variables|SKYLIGHT|GetSkylight%20Cast%20Shadow))
      (Class|LightComponentBase|SetCastRaytracedShadow _skylight (Variables|SKYLIGHT|GetSkylight%20Cast%20Raytraced%20Shadow))
      (Rendering|Components|Light|SetIntensity _skylight (Variables|SKYLIGHT|GetSkylight%20Intensity))
      (Class|SkyLightComponent|SetVolumetricScatteringIntensity _skylight (Variables|SKYLIGHT|GetSkylight%20Volumetric%20Intensity))
      (Rendering|Components|Light|SetLightColor _skylight (Variables|SKYLIGHT|GetSkylight%20Color))
      (Class|SkyLightComponent|SetIndirectLightingIntensity _skylight (Variables|SKYLIGHT|GetSkylight%20Indirect%20Lighting%20Intensity))
      (Class|LightComponentBase|SetSamplesPerPixel _skylight (Variables|SKYLIGHT|GetSkylight%20Raytrace%20Samples%20Per%20Pixel))
      (Class|LightComponentBase|SetAffectReflection _skylight (Variables|SKYLIGHT|GetSkylight%20Affect%20Reflections))
      (Class|SkyLightComponent|SetLowerHemisphereColor _skylight (Variables|SKYLIGHT|GetSkylight%20Lower%20Hemisphere%20Color))
      (Class|LightComponentBase|SetCastVolumetricShadow _skylight (Variables|SKYLIGHT|GetSkylight%20Cast%20Volumetric%20Shadow))
      (Rendering|SetVisibility _skylight (Variables|SKYLIGHT|GetSkylight%20Visibility) false)
      (Class|SkyLightComponent|RecaptureSky _skylight))
    (:then_2
      ;[1 1 1] Exponential Height Fog
      (Class|ExponentialHeightFogComponent|SetFogDensity _exponentialheightfog (Variables|EXPONENTIALHEIGHTFOG|GetExponential%20Fog%20Density))
      (Class|ExponentialHeightFogComponent|SetFogHeightFalloff _exponentialheightfog (Variables|EXPONENTIALHEIGHTFOG|GetExponential%20Fog%20Height%20Falloff))
      (Class|ExponentialHeightFogComponent|SetFogInscatteringColor _exponentialheightfog (Variables|EXPONENTIALHEIGHTFOG|GetExponential%20Fog%20Inscattering%20Color))
      (Class|ExponentialHeightFogComponent|SetFogMaxOpacity _exponentialheightfog (Variables|EXPONENTIALHEIGHTFOG|GetExponential%20Fog%20Max%20Opacity))
      (Class|ExponentialHeightFogComponent|SetStartDistance _exponentialheightfog (Variables|EXPONENTIALHEIGHTFOG|GetExponential%20Fog%20Start%20Distance))
      (Class|ExponentialHeightFogComponent|SetFogCutoffDistance _exponentialheightfog (Variables|EXPONENTIALHEIGHTFOG|GetExponential%20Fog%20Cutoff%20Distance))
      (Class|ExponentialHeightFogComponent|SetInscatteringColorCubemap _exponentialheightfog (Variables|EXPONENTIALHEIGHTFOG|GetExponential%20Fog%20Inscattering%20Cube%20Map))
      (Class|ExponentialHeightFogComponent|SetInscatteringColorCubemapAngle _exponentialheightfog (Variables|EXPONENTIALHEIGHTFOG|GetExponential%20Cube%20Map%20Angle))
      (Class|ExponentialHeightFogComponent|SetInscatteringTextureTint _exponentialheightfog (Variables|EXPONENTIALHEIGHTFOG|GetExponential%20Cubemap%20Tint))
      (Class|ExponentialHeightFogComponent|SetDirectionalInscatteringExponent _exponentialheightfog (Variables|EXPONENTIALHEIGHTFOG|GetExponential%20Inscattering%20Exponent))
      (Class|ExponentialHeightFogComponent|SetDirectionalInscatteringStartDistance _exponentialheightfog (Variables|EXPONENTIALHEIGHTFOG|GetExponential%20Inscattering%20Start%20Distance))
      (Class|ExponentialHeightFogComponent|SetDirectionalInscatteringColor _exponentialheightfog (Variables|EXPONENTIALHEIGHTFOG|GetExponential%20Directional%20Inscattering%20Color))
      (Class|ExponentialHeightFogComponent|SetVolumetricFog _exponentialheightfog (Variables|EXPONENTIALHEIGHTFOG|GetEnable%20Volumetrics))
      (Class|ExponentialHeightFogComponent|SetVolumetricFogScatteringDistribution _exponentialheightfog (Variables|EXPONENTIALHEIGHTFOG|GetVolumetric%20Scattering%20Distrubition))
      (Class|ExponentialHeightFogComponent|SetVolumetricFogAlbedo _exponentialheightfog (Variables|EXPONENTIALHEIGHTFOG|GetVolumetric%20Albedo))
      (Class|ExponentialHeightFogComponent|SetVolumetricFogEmissive _exponentialheightfog (Variables|EXPONENTIALHEIGHTFOG|GetVolumetric%20Emissive))
      (Class|ExponentialHeightFogComponent|SetVolumetricFogExtinctionScale _exponentialheightfog (Variables|EXPONENTIALHEIGHTFOG|GetVolumetric%20Extinction%20Scale))
      (Class|ExponentialHeightFogComponent|SetVolumetricFogDistance _exponentialheightfog (Variables|EXPONENTIALHEIGHTFOG|GetVolumetric%20View%20Distance))
      (Rendering|SetVisibility _exponentialheightfog (Variables|EXPONENTIALHEIGHTFOG|GetExponential%20Visibility) false)
      ;[1 1 1] Post Process
      (Variables|/Script/Engine.PostProcessComponent|SetSettings (Variables|Default|GetPostProcess) (Variables|POSTPROCESS|GetPost%20Process%20Settings)))))